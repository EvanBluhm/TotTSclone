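; BaDaunte is a barrel hazard actor that slides back and forth and damages whatever it hits.
; From BeginPlay, a self-calling Roll event chains two eased, latent MoveComponentTo moves, looping endlessly.
; MoveFoward and MoveBackward offset the barrel's current relative X by MoveDistance in opposite directions, keeping its rotation unchanged.
; The Hit event applies BarrelDamage to the other actor without filtering.
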(event `Roll`
  ;[0.2257 1 0] Barrel Rolls
  (`|ExecutionSequence`
    (:`then_0`
      (bind (_returnvalue _relative_rotation) (`self.move foward` (`self.Barrel`)))
      (`KismetSystemLibrary.MoveComponentTo` (`self.Barrel`) _returnvalue _relative_rotation true true 3.0)
      (bind (_returnvalue_2 _relative_rotation_2) (`self.move backward` (`self.Barrel`)))
      (`KismetSystemLibrary.MoveComponentTo` (`self.Barrel`) _returnvalue_2 _relative_rotation_2 true true 3.0)
      (`self.Roll`))))

(event `self.ReceiveBeginPlay`
  ;[0.2257 1 0] Barrel Rolls
  (`self.Roll`))

(event `self.ReceiveHit`
  (params (MyComp :type "PrimitiveComponent Object Reference") (Other :type "Actor Object Reference") (OtherComp :type "PrimitiveComponent Object Reference") (bSelfMoved :type Boolean) (HitLocation :type "Vector Structure") (HitNormal :type "Vector Structure") (NormalImpulse :type "Vector Structure") (Hit :type "HitResult Structure (by ref)"))
  (`GameplayStatics.ApplyDamage` Other (`self.barrel damage`)))

(fn `move backward`
  (params (Mesh :type "StaticMeshComponent Object Reference"))
  (returns (ReturnValue :type "Vector Structure") (`Relative Rotation` :type "Rotator Structure"))
  (bind (_relativelocation_x _relativelocation_y _relativelocation_z) (`KismetMathLibrary.BreakVector` (`SceneComponent.RelativeLocation` Mesh)))
  (return (`KismetMathLibrary.MakeVector` (+ (`self.move distance`) _relativelocation_x) _relativelocation_y _relativelocation_z) (`SceneComponent.RelativeRotation` Mesh)))

(fn `move foward`
  (params (Mesh :type "StaticMeshComponent Object Reference"))
  (returns (ReturnValue :type "Vector Structure") (`Relative Rotation` :type "Rotator Structure"))
  (bind (_relativelocation_x _relativelocation_y _relativelocation_z) (`KismetMathLibrary.BreakVector` (`SceneComponent.RelativeLocation` Mesh)))
  (return (`KismetMathLibrary.MakeVector` (- _relativelocation_x (`self.move distance`)) _relativelocation_y _relativelocation_z) (`SceneComponent.RelativeRotation` Mesh)))

(fn `UserConstructionScript`)