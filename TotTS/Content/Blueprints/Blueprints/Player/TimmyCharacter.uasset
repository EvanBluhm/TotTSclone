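; Top-down player character with axis movement, sprint, impulse-based roll, melee attacks, damage handling and a pause menu toggle.
; Sprint, roll and attacks spend Stamina, then feed a shared regen loop that waits for Stamina to settle and refills faster when standing still.
; The equipped Helmet child actor supplies speed, health, stamina and muscle bonuses, with muscle boosting the Weapon child actor's damage.
; Secondary attack currently only spends stamina.
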(event `InputAction|Sprint`
  (params (Key :type "Key Structure"))
  (bind _charactermovement (`self.CharacterMovement`))
  (bind _stamina (`self.stamina`))
  (bind _ashelmet_base (cast `/Game/Blueprints/Blueprints/Helmets/HelmetBase` (`ChildActorComponent.ChildActor` (`self.Helmet`)) :!pure true))
  (bind _speedincrease (`/Game/Blueprints/Blueprints/Helmets/HelmetBase.SpeedIncrease` _ashelmet_base))
  ;[0 1 0.1094] Stamina Drain
  (:`Pressed`
    (set `CharacterMovementComponent.MaxWalkSpeed` (+ 500.0 _speedincrease) _charactermovement)
    (bind _output_get (set `self.Sprinting` true))
    (if (and (`KismetMathLibrary.NotEqualExactly_VectorVector` (`self.GetVelocity`)) (>= _stamina 0.0) _output_get) :!label _label
      (set `self.stamina` (- _stamina 0.001))
      (`KismetSystemLibrary.Delay` 0.008)
      (goto _label)
      (else
        (set `CharacterMovementComponent.MaxWalkSpeed` (+ 300.0 _speedincrease) _charactermovement :!label _label_2)
        (set `self.Sprinting` false)
        (`self.Stamina Regen` (`/Game/Blueprints/Blueprints/Helmets/HelmetBase.StaminaIncrease` _ashelmet_base) :!label _label_3))))
  (:`Released`
    (goto _label_2)))

(event `InputAction|Roll`
  (params (Key :type "Key Structure"))
  (bind _returnvalue (`self.GetVelocity`))
  (bind _charactermovement (`self.CharacterMovement`))
  (bind _stamina (`self.stamina`))
  ;[0 1 0.1094] Stamina Drain
  (:`Pressed`
    (if (>= _stamina 0.25)
      (set `self.Rolling` true)
      (`/Engine/EditorBlueprintResources/StandardMacros.DoOnce` false :!label _label_4
        (:`Completed`
          (if (== _returnvalue (0.0 0.0 0.0))
            (`CharacterMovementComponent.AddImpulse` _charactermovement (* (`KismetMathLibrary.GetForwardVector` (`self.K2_GetActorRotation`)) 6000.0) true)
            (else
              (`CharacterMovementComponent.AddImpulse` _charactermovement (* _returnvalue 30.0) true)))
          (set `self.stamina` (- _stamina 0.25))
          (`|ExecutionSequence`
            (:`then_0`
              (set `self.Rolling` false))
            (:`then_1`
              (`KismetSystemLibrary.Delay` 0.5)
              (goto _label_4 :!via `Reset`)))))))
  (:`Released`
    (goto _label_3)))

(event `InputAction|Attack Main`
  (params (Key :type "Key Structure"))
  (bind _stamina (`self.stamina`))
  (bind _asmelee_base (cast `/Game/Blueprints/Blueprints/MeleeWeaponry/MeleeBase` (`ChildActorComponent.ChildActor` (`self.Weapon`)) :!pure true))
  ;[0 1 0.1094] Stamina Drain
  (:`Pressed`
    (if (>= _stamina 0.01)
      (`/Engine/EditorBlueprintResources/StandardMacros.DoOnce` false :!label _label_5
        (:`Completed`
          (set `self.stamina` (- _stamina 0.01))
          (set `/Game/Blueprints/Blueprints/MeleeWeaponry/MeleeBase.Damage Amount` (+ (`/Game/Blueprints/Blueprints/MeleeWeaponry/MeleeBase.Base Damage` _asmelee_base) (`/Game/Blueprints/Blueprints/Helmets/HelmetBase.Muscle` (cast `/Game/Blueprints/Blueprints/Helmets/HelmetBase` (`ChildActorComponent.ChildActor` (`self.Helmet`)) :!pure true))) _asmelee_base)
          (`/Game/Blueprints/Blueprints/MeleeWeaponry/MeleeBase.weaponActive` _asmelee_base)
          (`KismetSystemLibrary.Delay` 0.05)
          (`/Game/Blueprints/Blueprints/MeleeWeaponry/MeleeBase.weaponInactive` _asmelee_base)
          (goto _label_5 :!via `Reset`)))))
  (:`Released`
    (goto _label_3)))

(event `InputAction|Attack Alt`
  (params (Key :type "Key Structure"))
  (bind _stamina (`self.stamina`))
  ;[0 1 0.1094] Stamina Drain
  (:`Pressed`
    (if (>= _stamina 0.1)
      (`/Engine/EditorBlueprintResources/StandardMacros.DoOnce` false :!label _label_6
        (:`Completed`
          (set `self.stamina` (- _stamina 0.1))
          (`KismetSystemLibrary.Delay` 0.1)
          (goto _label_6 :!via `Reset`)))))
  (:`Released`
    (goto _label_3)))

(event `InputAxis|Move Up/Down`
  (params (AxisValue :type "Float (single-precision)"))
  ;[0 0.5547 1] Movement
  (`self.AddMovementInput` (1.0 0.0 0.0) AxisValue))

(event `InputAxis|Move Left/Right`
  (params (AxisValue :type "Float (single-precision)"))
  ;[0 0.5547 1] Movement
  (`self.AddMovementInput` (0.0 1.0 0.0) AxisValue))

(event `self.ReceiveBeginPlay`
  (set `CharacterMovementComponent.MaxWalkSpeed` (+ 300.0 (`/Game/Blueprints/Blueprints/Helmets/HelmetBase.SpeedIncrease` (cast `/Game/Blueprints/Blueprints/Helmets/HelmetBase` (`ChildActorComponent.ChildActor` (`self.Helmet`)) :!pure true))) (`self.CharacterMovement`))
  ;[0.5937 1 0] Create UI
  (bind _returnvalue (`|CreateWidget` "/Game/Blueprints/UserInterface/TopDownUI.TopDownUI_C"))
  (`UserWidget.AddToViewport` _returnvalue 0)
  ;[0.9219 0 1] Set Weapon Owner
  (`self.SetOwner` (`ChildActorComponent.ChildActor` (`self.Weapon`)) self))

(event `self.ReceiveAnyDamage`
  (params (Damage :type "Float (single-precision)") (DamageType :type "DamageType Object Reference") (InstigatedBy :type "Controller Object Reference") (DamageCauser :type "Actor Object Reference"))
  ;[1 0.2578 0] Take Damage
  (if (not (`self.Rolling`))
    (bind _output_get (set `self.CurrentHealth` (- (+ (`self.CurrentHealth`) (`/Game/Blueprints/Blueprints/Helmets/HelmetBase.HealthIncrease` (cast `/Game/Blueprints/Blueprints/Helmets/HelmetBase` (`ChildActorComponent.ChildActor` (`self.Helmet`)) :!pure true))) Damage))))
  (`KismetSystemLibrary.PrintString` (`KismetStringLibrary.Conv_DoubleToString` _output_get)))

(event `InputAction|Pause` :consume false :paused true
  (params (Key :type "Key Structure"))
  (:`Pressed`
    (`/Engine/EditorBlueprintResources/StandardMacros.FlipFlop`
      (:`A`
        (`GameplayStatics.SetGamePaused` true)
        (bind _returnvalue (`|CreateWidget` "/Game/Blueprints/UserInterface/PauseMenu.PauseMenu_C"))
        (`UserWidget.AddToViewport` _returnvalue 0))
      (:`B`
        (`GameplayStatics.SetGamePaused` false)
        (`Widget.RemoveFromParent` _returnvalue)))))

(fn `UserConstructionScript`)