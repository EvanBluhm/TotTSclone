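; Player controller for Timmy that shows a movement tutorial widget prompting WASD use at BeginPlay.
; Move axis events feed four DoOnce gates, split on negative versus non-negative values, so zero input also counts as a direction.
; Each gate increments a counter, and a 0.1-second Delay loop polls it to clear the text at four.
; Main and alt attack inputs end in DoOnce nodes with no further logic.
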(event `self.ReceiveBeginPlay`
  (bind __ (`self.!`))
  ;[0.5482 1 0.3152] Tutorial
  ;;[1 0 0.375] Movement
  (bind _returnvalue (`|CreateWidget` "/Game/Blueprints/Tutorial.Tutorial_C"))
  (`UserWidget.AddToViewport` _returnvalue 0)
  (set `/Game/Blueprints/Tutorial.TutorialText` "Use 'WASD' Keys to Move" _returnvalue)
  (`|ExecutionSequence`
    (:`then_0`
      (goto _label_2 :!via `Reset`))
    (:`then_1`
      (goto _label_3 :!via `Reset`))
    (:`then_2`
      (goto _label_5 :!via `Reset`))
    (:`then_3`
      (goto _label_6 :!via `Reset`))
    (:`then_4`
      (if (== __ 4) :!label _label
        (set `/Game/Blueprints/Tutorial.TutorialText` "" _returnvalue)
        (else
          (`KismetSystemLibrary.Delay` 0.1)
          (goto _label))))))

(event `InputAction|Roll` :consume false
  (params (Key :type "Key Structure"))
  ;[0.5482 1 0.3152] Tutorial
)

(event `InputAxis|Move Up/Down` :consume false
  (params (AxisValue :type "Float (single-precision)"))
  ;[0.5482 1 0.3152] Tutorial
  ;;[1 0 0.375] Movement
  (if (< AxisValue 0.0)
    (`/Engine/EditorBlueprintResources/StandardMacros.DoOnce` true :!label _label_2
      (:`Completed`
        _))
    (else
      (`/Engine/EditorBlueprintResources/StandardMacros.DoOnce` true :!label _label_3
        (:`Completed`
          _))))
  (set `self.!` (+ (`self.!`) 1) :!label _label_4))

(event `InputAction|Sprint` :consume false
  (params (Key :type "Key Structure"))
  ;[0.5482 1 0.3152] Tutorial
)

(event `InputAxis|Move Left/Right` :consume false
  (params (AxisValue :type "Float (single-precision)"))
  ;[0.5482 1 0.3152] Tutorial
  ;;[1 0 0.375] Movement
  (if (< AxisValue 0.0)
    (`/Engine/EditorBlueprintResources/StandardMacros.DoOnce` true :!label _label_5
      (:`Completed`
        (goto _label_4)))
    (else
      (`/Engine/EditorBlueprintResources/StandardMacros.DoOnce` true :!label _label_6
        (:`Completed`
          (goto _label_4))))))

(event `InputAction|Attack Main` :consume false
  (params (Key :type "Key Structure"))
  ;[0.5482 1 0.3152] Tutorial
  (:`Pressed`
    (`/Engine/EditorBlueprintResources/StandardMacros.DoOnce` true)))

(event `InputAction|Attack Alt` :consume false
  (params (Key :type "Key Structure"))
  ;[0.5482 1 0.3152] Tutorial
  (:`Pressed`
    (`/Engine/EditorBlueprintResources/StandardMacros.DoOnce` true)))

(fn `UserConstructionScript`)