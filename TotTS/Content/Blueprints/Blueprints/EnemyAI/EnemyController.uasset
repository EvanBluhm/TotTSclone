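; Enemy AI controller that runs the BT_Enemy behavior tree on possession and writes the line-of-sight flag and target to its blackboard.
; Both begin and end overlap mark TopDownCharacter as the seen target, while Tick randomly clears the sight flag after random delays.
; The sight perception event is empty; its player-tag check, startup grace period and timed loss of target sit in unconnected logic that never runs.
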(event `BeginOverlap`
  (bind _blackboard (`self.Blackboard`))
  (`BlackboardComponent.SetValueAsBool` _blackboard (`self.HasLineOfSight`) true)
  (`BlackboardComponent.SetValueAsObject` _blackboard (`self.EnemyActor`) "/Game/Blueprints/Blueprints/TopDownCharacter.TopDownCharacter"))

(event `EndOverlap`
  (bind _blackboard (`self.Blackboard`))
  (`BlackboardComponent.SetValueAsBool` _blackboard (`self.HasLineOfSight`) true)
  (`BlackboardComponent.SetValueAsObject` _blackboard (`self.EnemyActor`) "/Game/Blueprints/Blueprints/TopDownCharacter.TopDownCharacter"))

(event `self.SightRange.OnTargetPerceptionUpdated`
  (params (Actor :type "Actor Object Reference") (Stimulus :type "AIStimulus Structure")))

(event `self.ReceiveBeginPlay`
  (`KismetSystemLibrary.Delay` 1.0)
  (bind _output_get (set `self.GracePerioid ` true)))

(event `StartEnemyTimer`
  (bind _blackboard (`self.Blackboard`))
  (`BlackboardComponent.SetValueAsBool` _blackboard (`self.HasLineOfSight`) false)
  (`BlackboardComponent.SetValueAsObject` _blackboard (`self.EnemyActor`) null))

(event `self.ReceivePossess`
  (params (PossessedPawn :type "Pawn Object Reference"))
  (`self.RunBehaviorTree` "/Game/Blueprints/Blueprints/EnemyAI/BT_Enemy.BT_Enemy"))

(event `self.ReceiveTick`
  (params (DeltaSeconds :type "Float (single-precision)"))
  (`KismetSystemLibrary.Delay` (`KismetMathLibrary.RandomFloat`))
  (if (== (`KismetMathLibrary.RandomIntegerInRange` 0 100) 1)
    (`KismetSystemLibrary.K2_ClearAndInvalidateTimerHandle` (`self.EnemyTimer`))
    (`BlackboardComponent.SetValueAsBool` (`self.Blackboard`) (`self.HasLineOfSight`) false)))

(fn `UserConstructionScript`)