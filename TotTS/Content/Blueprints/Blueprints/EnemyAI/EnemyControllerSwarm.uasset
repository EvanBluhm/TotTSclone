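; AI controller for swarm enemies that runs the BT_Enemy behavior tree on possess and feeds its Blackboard with player-detection state.
; BeginOverlap sets the player as EnemyActor if line of sight passes and cancels the forget timer.
; EndOverlap starts that timer, which clears sight and target after LineOfSightTimer elapses.
; Retreat flags IsRetreating and drops line of sight.
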(event `BeginOverlap`
  (bind _blackboard (`self.Blackboard`))
  (if (`self.LineOfSightTo` (`GameplayStatics.GetPlayerPawn` 0))
    (`KismetSystemLibrary.K2_ClearAndInvalidateTimerHandle` (`self.EnemyTimer`))
    (`BlackboardComponent.SetValueAsBool` _blackboard (`self.HasLineOfSight`) true)
    (`BlackboardComponent.SetValueAsObject` _blackboard (`self.EnemyActor`) (`GameplayStatics.GetPlayerCharacter` 0))))

(event `EndOverlap`
  (bind _returnvalue (`KismetSystemLibrary.K2_SetTimerDelegate` (delegate `StartEnemyTimer`) (`self.LineOfSightTimer`)))
  (set `self.EnemyTimer` _returnvalue))

(event `StartEnemyTimer`
  (bind _blackboard (`self.Blackboard`))
  (`BlackboardComponent.SetValueAsBool` _blackboard (`self.HasLineOfSight`) false)
  (`BlackboardComponent.SetValueAsObject` _blackboard (`self.EnemyActor`) null))

(event `self.ReceivePossess`
  (params (PossessedPawn :type "Pawn Object Reference"))
  (`self.RunBehaviorTree` "/Game/Blueprints/Blueprints/EnemyAI/BT_Enemy.BT_Enemy"))

(event `Retreat`
  (bind _blackboard (`self.Blackboard`))
  (`BlackboardComponent.SetValueAsBool` _blackboard (`self.IsRetreating`) true)
  (`BlackboardComponent.SetValueAsBool` _blackboard (`self.HasLineOfSight`) false))

(fn `UserConstructionScript`)