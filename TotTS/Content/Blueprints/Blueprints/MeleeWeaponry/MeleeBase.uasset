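; MeleeBase is a melee weapon base Blueprint that damages actors its collision component overlaps.
; weaponActive and weaponInactive events turn the hitbox on with an OverlapAll profile and off by disabling collision.
; Overlaps with actors of the owner's own class are ignored; others take DamageAmount damage.
; A DoOnce with a short delayed reset throttles repeat hits to one at a time across all targets.
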(event `self.CollisionDetection.OnComponentBeginOverlap`
  (params (OverlappedComponent :type "PrimitiveComponent Object Reference") (OtherActor :type "Actor Object Reference") (OtherComp :type "PrimitiveComponent Object Reference") (OtherBodyIndex :type Integer) (bFromSweep :type Boolean) (SweepResult :type "HitResult Structure (by ref)"))
  (if (!= (`GameplayStatics.GetObjectClass` OtherActor) (`GameplayStatics.GetObjectClass` (`self.GetOwner`)))
    (`/Engine/EditorBlueprintResources/StandardMacros.DoOnce` false :!label _label
      (:`Completed`
        (`GameplayStatics.ApplyDamage` OtherActor (`self.damageAmount`))
        (`KismetSystemLibrary.Delay` 0.05)
        (goto _label :!via `Reset`)))))

(event `weaponActive`
  (`PrimitiveComponent.SetCollisionProfileName` (`self.CollisionDetection`) "OverlapAll" true))

(event `weaponInactive`
  (`PrimitiveComponent.SetCollisionEnabled` (`self.CollisionDetection`) "NoCollision"))

(fn `UserConstructionScript`)