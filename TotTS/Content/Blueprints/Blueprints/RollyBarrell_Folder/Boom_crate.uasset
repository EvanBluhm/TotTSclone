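; Boom_crate is an explosive crate that damages everything nearby when destroyed.
; AnyDamage subtracts incoming damage from CrateHealth and triggers the blast once health drops below zero.
; A DoOnce gate limits the blast to a single run, which applies massive fixed damage to every actor overlapping the Radius component, then destroys the crate.
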(event `self.ReceiveAnyDamage`
  (params (Damage :type "Float (single-precision)") (DamageType :type "DamageType Object Reference") (InstigatedBy :type "Controller Object Reference") (DamageCauser :type "Actor Object Reference"))
  (bind _output_get (set `self.Crate health` (- (`self.Crate health`) Damage)))
  (if (< _output_get 0.0)
    (`/Engine/EditorBlueprintResources/StandardMacros.DoOnce` false
      (:`Completed`
        (for _array_element (`PrimitiveComponent.GetOverlappingActors` (`self.radius`) null)
          (`GameplayStatics.ApplyDamage` _array_element 12345678.0))
        (`self.K2_DestroyActor`)))))

(fn `UserConstructionScript`)