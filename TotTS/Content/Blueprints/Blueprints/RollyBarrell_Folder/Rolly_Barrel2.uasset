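; Rolly barrel actor that moves its Barrel component back and forth along relative X, starting at BeginPlay.
; The Roll event chains two latent MoveComponentTo calls, an eased four-second move toward negative X and a linear three-second return, then calls itself to loop.
; Helper functions offset the current location by MoveDistance and pass rotation through unchanged, so the barrel translates without spinning.
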(event `Roll`
  (`|ExecutionSequence`
    (:`then_0`
      (bind (_returnvalue _relative_rotation) (`self.move foward` (`self.Barrel`)))
      (`KismetSystemLibrary.MoveComponentTo` (`self.Barrel`) _returnvalue _relative_rotation true true 4.0)
      (bind (_returnvalue_2 _relative_rotation_2) (`self.move backward` (`self.Barrel`)))
      (`KismetSystemLibrary.MoveComponentTo` (`self.Barrel`) _returnvalue_2 _relative_rotation_2 false false 3.0)
      (`self.Roll`))))

(event `self.ReceiveBeginPlay`
  (`self.Roll`))

(fn `move backward`
  (params (Mesh :type "StaticMeshComponent Object Reference"))
  (returns (ReturnValue :type "Vector Structure") (`Relative Rotation` :type "Rotator Structure"))
  (bind (_relativelocation_x _relativelocation_y _relativelocation_z) (`KismetMathLibrary.BreakVector` (`SceneComponent.RelativeLocation` Mesh)))
  (return (`KismetMathLibrary.MakeVector` (+ (`self.move distance`) _relativelocation_x) _relativelocation_y _relativelocation_z) (`SceneComponent.RelativeRotation` Mesh)))

(fn `move foward`
  (params (Mesh :type "StaticMeshComponent Object Reference"))
  (returns (ReturnValue :type "Vector Structure") (`Relative Rotation` :type "Rotator Structure"))
  (bind (_relativelocation_x _relativelocation_y _relativelocation_z) (`KismetMathLibrary.BreakVector` (`SceneComponent.RelativeLocation` Mesh)))
  (return (`KismetMathLibrary.MakeVector` (- _relativelocation_x (`self.move distance`)) _relativelocation_y _relativelocation_z) (`SceneComponent.RelativeRotation` Mesh)))

(fn `UserConstructionScript`)